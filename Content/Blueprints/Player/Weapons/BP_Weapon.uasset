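; BP_Weapon is a short-lived projectile that damages enemies and the player and destroys barriers.
; When its sphere begins overlapping a barrier, it spawns a small Niagara fire explosion and destroys the barrier.
; Other overlaps cast to BP_Enemy, then BP_Player, to apply fixed damage, without destroying the projectile.
; It destroys itself after a short delay, or sooner if Tick finds its movement speed has dropped below a threshold.
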(event OnComponentEndOverlap(Sphere1)
  (params (OverlappedComponent :type Primitive%20Component%20Object%20Reference) (OtherActor :type Actor%20Object%20Reference) (OtherComp :type Primitive%20Component%20Object%20Reference) (OtherBodyIndex :type Integer))
  ;[1 1 1] Overlap
  (Utilities|FlowControl|DoOnce false ; enters at Reset
    (:Completed
      (bind _asbp_enemy (Utilities|Casting|CastToBP_Enemy (stale OnComponentBeginOverlap(Sphere1) OtherActor))
        (:then
          (Default|DamageEnemy _asbp_enemy 17))
        (:CastFailed
          (bind _asbp_player (Utilities|Casting|CastToBP_Player (stale OnComponentBeginOverlap(Sphere1) OtherActor)))
          (Default|ApplyDamage _asbp_player 20))))))

(event OnComponentBeginOverlap(Sphere1)
  (params (OverlappedComponent :type Primitive%20Component%20Object%20Reference) (OtherActor :type Actor%20Object%20Reference) (OtherComp :type Primitive%20Component%20Object%20Reference) (OtherBodyIndex :type Integer) (bFromSweep :type Boolean) (SweepResult :type Hit%20Result%20Structure%20%28by%20ref%29))
  ;[1 1 1] Overlap
  (bind _asbp_barrier (Utilities|Casting|CastToBP_Barrier OtherActor)
    (:then
      (Niagara|SpawnSystematLocation "/Game/M5VFXVOL2/Niagara/Explosion/NFire_Exp_01.NFire_Exp_01" (Transformation|GetActorLocation _asbp_barrier) "0, 0, 0" "0.050000,0.050000,0.050000")
      (Actor|DestroyActor _asbp_barrier))
    (:CastFailed
      (bind _asbp_enemy (Utilities|Casting|CastToBP_Enemy OtherActor)
        (:then
          (Default|DamageEnemy _asbp_enemy 17))
        (:CastFailed
          (bind _asbp_player (Utilities|Casting|CastToBP_Player OtherActor))
          (Default|ApplyDamage _asbp_player 20))))))

(event EventBeginPlay
  ;[1 1 1] Begin Play
  (Utilities|FlowControl|Delay 3.0)
  (Actor|DestroyActor))

(event EventTick
  (params (DeltaSeconds :type Float%20%28single-precision%29))
  ;[1 1 1] Tick
  (if (<= (Math|Vector|VectorLength (Variables|/Script/Engine.MovementComponent|GetVelocity (Variables|Default|GetProjectileMovement))) 1.5e+02)
    (Actor|DestroyActor)))

(fn ConstructionScript)