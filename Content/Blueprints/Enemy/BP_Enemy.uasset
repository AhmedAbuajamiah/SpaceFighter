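; Enemy actor that chases a seen player, fires BP_Weapon bursts and has regenerating health.
; Pawn sensing aims an arrow, interpolates movement toward the player and triggers randomly cooled-down bursts unless the player is higher.
; Tick starts timer-based healing after a damage-free delay, though the health-cap check calls an empty stop function.
; Damage interrupts healing or destroys the enemy with a Niagara explosion, and BeginPlay links its health widget.
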(event OnSeePawn(PawnSensing)
  (params (Pawn :type Pawn%20Object%20Reference))
  (bind _scene (Variables|Default|GetScene))
  (bind _returnvalue (Transformation|GetWorldRotation _scene))
  ;[1 1 1] PawnSense
  (bind _asbp_player (Utilities|Casting|CastToBP_Player Pawn))
  (Transformation|SetWorldRotation (Variables|Default|GetArrow1) (Math|Rotator|FindLookatRotation (Transformation|GetActorLocation) (Transformation|GetActorLocation _asbp_player)) false false)
  (Utilities|FlowControl|Sequence
    (:then_0
      (CallFunction|Moveto)
      (Variables|Default|SetMoveToLocation (+ (Transformation|GetActorLocation _asbp_player) "0.000000,0.000000,50.000000")))
    (:then_1
      (Utilities|FlowControl|DoOnce false :!label _label
        (:Completed
          (if (not (> (.z (Transformation|GetActorLocation _asbp_player)) (.z (Transformation|GetActorLocation))))
            (for _index (range 0 3)
              (Game|SpawnActorfromClass "/Game/Blueprints/Player/Weapons/BP_Weapon.BP_Weapon_C" (Math|Transform|MakeTransform (Transformation|GetWorldLocation _scene) (Math|Rotator|CombineRotators _returnvalue (Math|Rotator|SelectRotator "0.000000,0.000000,90.000000" "0.000000,0.000000,-90.000000" (> (.Roll (Math|Rotator|BreakRotator _returnvalue)) 0.0))) "1.000000,1.000000,1.000000") "Undefined" "MultiplyWithRoot" 0 0)
              (Utilities|FlowControl|Delay 0.2))
            (Utilities|FlowControl|Delay (Math|Random|RandomFloatinRange 1.5 4.0))
            (goto _label Reset)))))))

(event Custom|DamageEnemy
  (params (Damage :type Integer))
  ;[1 1 1] Take Damage
  (bind _output_get (Variables|Default|SetHealth (- (Variables|Default|GetHealth) Damage)))
  (if (< _output_get 1)
    (Niagara|SpawnSystematLocation "/Game/M5VFXVOL2/Niagara/Explosion/NFire_Exp_01.NFire_Exp_01" (Transformation|GetActorLocation) "0, 0, 0" "0.100000,0.100000,0.100000")
    (Actor|DestroyActor)
    (else
      (Variables|Default|SetLastTakenDamaage (.Seconds (Class|GameplayStatics|GetAccurateRealTime))))))

(event Custom|HealthTimer_Event
  ;[1 1 1] ChargeHealth
  (bind _output_get (Variables|Default|SetHealth (Math|Float|Truncate (Math|Interpolation|FInterpTo (Math|Conversions|ToFloat(Integer) (Variables|Default|GetHealth)) (Math|Conversions|ToFloat(Integer) (+ (Variables|Default|GetHealth) 20)) (Utilities|Time|GetWorldDeltaSeconds) 0.0))))
  (if (not (<= _output_get 100))
    (CallFunction|StopChargingHeat)))

(event Custom|Charge_Health
  ;[1 1 1] ChargeHealth
  (bind _returnvalue (Utilities|Time|SetTimerbyEvent (delegate Custom|HealthTimer_Event) 0.3 true false 0.5))
  (Variables|Default|SetHealthTimer _returnvalue))

(event Custom|StopChargingHealth
  ;[1 1 1] ChargeHealth
  (Utilities|Time|ClearandInvalidateTimerbyHandle (Variables|Default|GetHealthTimer)))

(event EventBeginPlay
  ;[1 1 1] BeginPlay
  (bind _aswbp_enemy_health (Utilities|Casting|CastToWBP_EnemyHealth (UserInterface|GetUserWidgetObject (Variables|Default|GetWidget))))
  (Variables|/Game/Blueprints/Enemy/WBP_EnemyHealth.WBP_EnemyHealth_C|SetEnemy _aswbp_enemy_health self)
  (Utilities|FlowControl|Delay 2.0)
  (Variables|Default|SetMoveToLocation (Transformation|GetActorLocation)))

(event EventTick
  (params (DeltaSeconds :type Float%20%28single-precision%29))
  ;[1 1 1] Tick
  (if (> (- (.Seconds (Class|GameplayStatics|GetAccurateRealTime)) (Variables|Default|GetLastTakenDamaage)) 2)
    (Utilities|FlowControl|DoOnce false :!label _label
      (:Completed
        (CallFunction|ChargeHealth)))
    (else
      (CallFunction|StopChargingHealth)
      (goto _label Reset))))

(fn ConstructionScript)

(fn Moveto
  (Transformation|SetActorLocation (Math|Interpolation|VInterpTo (Transformation|GetActorLocation) (Variables|Default|GetMoveToLocation) (Utilities|Time|GetWorldDeltaSeconds) 1.0) false false))

(fn StopChargingHeat)